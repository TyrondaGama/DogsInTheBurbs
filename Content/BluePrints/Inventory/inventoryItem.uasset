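; Inventory item actor that the ThirdPersonCharacter picks up, and that makes an AI-audible noise when it hits something else.
; Sphere overlap increments its Type count in the character's Inventory map, while mesh hit calls IncreaseThrowable and records LastPickup; both destroy the item.
; The first non-player hit plays a rubber chicken sound and reports noise with the player as instigator; every hit draws a debug sphere.
; The Throw function is empty.
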(event OnComponentBeginOverlap(Sphere)
  (params (OverlappedComponent :type Primitive%20Component%20Object%20Reference) (OtherActor :type Actor%20Object%20Reference) (OtherComp :type Primitive%20Component%20Object%20Reference) (OtherBodyIndex :type Integer) (bFromSweep :type Boolean) (SweepResult :type Hit%20Result%20Structure%20%28by%20ref%29))
  (bind _type (Variables|Default|GetType))
  (bind _asthird_person_character (Utilities|Casting|CastToThirdPersonCharacter OtherActor))
  (bind _output_get (Variables|Default|SetCurrentNumber (.Value (Utilities|Map|Find (Variables|/Game/ThirdPersonBP/Blueprints/ThirdPersonCharacter.ThirdPersonCharacter_C|GetInventory _asthird_person_character) _type))))
  (Utilities|Map|Remove (Variables|/Game/ThirdPersonBP/Blueprints/ThirdPersonCharacter.ThirdPersonCharacter_C|GetInventory _asthird_person_character) _type)
  (Utilities|Map|Add (Variables|/Game/ThirdPersonBP/Blueprints/ThirdPersonCharacter.ThirdPersonCharacter_C|GetInventory _asthird_person_character) _type (+ _output_get 1))
  (Actor|DestroyActor))

(event OnComponentHit(StaticMesh)
  (params (HitComponent :type Primitive%20Component%20Object%20Reference) (OtherActor :type Actor%20Object%20Reference) (OtherComp :type Primitive%20Component%20Object%20Reference) (NormalImpulse :type Vector :default "0, 0, 0") (Hit :type Hit%20Result%20Structure%20%28by%20ref%29))
  (bind _asthird_person_character (Utilities|Casting|CastToThirdPersonCharacter OtherActor))
  (Default|IncreaseThrowable _asthird_person_character)
  (Actor|DestroyActor)
  (Variables|/Game/ThirdPersonBP/Blueprints/ThirdPersonCharacter.ThirdPersonCharacter_C|SetLastPickup _asthird_person_character (Variables|Default|GetClass)))

(event Collision|EventHit
  (params (MyComp :type Primitive%20Component%20Object%20Reference) (Other :type Actor%20Object%20Reference) (OtherComp :type Primitive%20Component%20Object%20Reference) (bSelfMoved :type Boolean) (HitLocation :type Vector :default "0, 0, 0") (HitNormal :type Vector :default "0, 0, 0") (NormalImpulse :type Vector :default "0, 0, 0") (Hit :type Hit%20Result%20Structure%20%28by%20ref%29))
  (bind _returnvalue (Game|GetPlayerCharacter 0))
  (Rendering|Debug|DrawDebugSphere HitLocation 1e+02 12 "(R=1.000000,G=1.000000,B=1.000000,A=1.000000)" 1.0)
  (if (!= Other _returnvalue)
    (Utilities|FlowControl|DoOnce false
      (:Completed
        (Audio|PlaySoundatLocation "/Game/BluePrints/Inventory/Audio/rubber-chicken_Drop_Cue.rubber-chicken_Drop_Cue" HitLocation "0, 0, 0" 1.0 1.0 0.0 0 0 0)
        (Class|AISenseHearing|ReportNoiseEvent (Transformation|GetActorLocation) 1e+02 _returnvalue 1e+03 "None")))))

(fn ConstructionScript)

(fn Throw)