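; Enemy Blueprint that roams, investigates perceived stimuli and chases the player, restarting the level on a catch.
; Random AIMoveTo roaming yields to AI Perception investigation, while PawnSensing sight starts a chase with audio that Tick fades out via CanSeeEnemy.
; Reaching the player sets Caught, starting a recursive short-delay loop that turns player and camera toward the enemy as a montage and fade precede the level reload.
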(event OnSeePawn(PawnSensing)
  (params (Pawn :type Pawn%20Object%20Reference))
  ;[1 1 1] Chase
  (bind _asthird_person_character (Utilities|Casting|CastToThirdPersonCharacter (Game|GetPlayerCharacter 0)))
  (if (not (Variables|Default|GetCaught?))
    (Utilities|FlowControl|Sequence
      (:then_0
        (Variables|Default|SetisSeeingPlayer true)
        (AI|AIMoveTo self "0, 0, 0" _asthird_person_character 5.0 false
          (:then
            (Utilities|FlowControl|DoOnce false
              (:Completed
                (Audio|Components|Audio|Play (Variables|Default|GetAudio) 0.0))))
          (:OnSuccess
            (CallFunction|CatchPlayer))))
      (:then_1
        (Utilities|FlowControl|RetriggerableDelay 0.5)
        (Variables|Default|SetCan%20See%20Enemy false)))))

(event OnTargetPerceptionUpdated(AIPerception)
  (params (Actor :type Actor%20Object%20Reference) (Stimulus :type AI%20Stimulus%20Structure))
  (bind (_age _expirationage _strength _stimuluslocation _receiverlocation _tag _bsuccessfullysensed) (Utilities|Struct|BreakAIStimulus Stimulus))
  ;[1 1 1] Investigate Sound
  (Utilities|Casting|CastToThirdPersonCharacter Actor)
  (if _bsuccessfullysensed
    (Variables|Default|SetInvestigating? true)
    (AI|AIMoveTo self _stimuluslocation 0 5e+02 false
      (:OnSuccess
        (Utilities|FlowControl|Delay 6.0)
        (CallFunction|RandomRoam)))))

(event OnComponentHit(Sphere)
  (params (HitComponent :type Primitive%20Component%20Object%20Reference) (OtherActor :type Actor%20Object%20Reference) (OtherComp :type Primitive%20Component%20Object%20Reference) (NormalImpulse :type Vector :default "0, 0, 0") (Hit :type Hit%20Result%20Structure%20%28by%20ref%29))
  ;[1 1 1] Catch Player
)

(event Custom|Catch%20Player
  (bind _returnvalue (Game|GetPlayerController 0))
  ;[1 1 1] Catch Player
  (Variables|Default|SetCaught? true)
  (Variables|Default|SetShouldLoop? true)
  (bind _asthird_person_character (Utilities|Casting|CastToThirdPersonCharacter (Game|GetPlayerCharacter 0)))
  (if (Variables|Default|GetCaught?)
    (Utilities|FlowControl|Delay 0.001)
    (Transformation|SetActorRotation _asthird_person_character (Math|Interpolation|RInterpTo (Transformation|GetActorRotation _asthird_person_character) (Math|Rotator|FindLookatRotation (Transformation|GetActorLocation _asthird_person_character) (Transformation|GetActorLocation)) (Utilities|Time|GetWorldDeltaSeconds) 5.0))
    (Pawn|SetControlRotation _returnvalue (Math|Interpolation|RInterpTo (Pawn|GetControlRotation _returnvalue :!class /Script/Engine.Controller) (Math|Rotator|FindLookatRotation (Transformation|GetActorLocation _asthird_person_character) (Transformation|GetActorLocation)) (Utilities|Time|GetWorldDeltaSeconds) 0.0))
    (CallFunction|RotationLoop)
    (Utilities|FlowControl|DoOnce false :!label _label
      (:Completed
        (Utilities|FlowControl|Sequence
          (:then_0
            (Animation|PlayAnimMontage "/Game/Mannequin/Animations/Caught.Caught" 1.0 "None")
            (Utilities|FlowControl|Delay 1.0)
            (CameraFades|StartCameraFade :self (Game|GetPlayerCameraManager 0) :ToAlpha 1.0 :Duration 2.0 :bShouldFadeAudio true :bHoldWhenFinished true)
            (Utilities|FlowControl|Delay 2.1)
            (bind _returnvalue_2 (Game|GetCurrentLevelName true))
            (Game|OpenLevel(byName) (Utilities|String|StringToName _returnvalue_2))
            (Variables|Default|SetCaught? false))
          (:then_1
            (Utilities|FlowControl|Delay 0.5)
            (Variables|Default|SetShouldLoop? false)
            (goto _label Reset)))))))

(event Custom|Rotation%20Loop
  (bind _returnvalue (Game|GetPlayerController 0))
  ;[1 1 1] Catch Player
  (if (Variables|Default|GetCaught?)
    (Utilities|FlowControl|Delay 0.001)
    (Transformation|SetActorRotation (stale Custom|Catch%20Player _asthird_person_character) (Math|Interpolation|RInterpTo (Transformation|GetActorRotation (stale Custom|Catch%20Player _asthird_person_character)) (Math|Rotator|FindLookatRotation (Transformation|GetActorLocation (stale Custom|Catch%20Player _asthird_person_character)) (Transformation|GetActorLocation)) (Utilities|Time|GetWorldDeltaSeconds) 5.0))
    (Pawn|SetControlRotation _returnvalue (Math|Interpolation|RInterpTo (Pawn|GetControlRotation _returnvalue :!class /Script/Engine.Controller) (Math|Rotator|FindLookatRotation (Transformation|GetActorLocation (stale Custom|Catch%20Player _asthird_person_character)) (Transformation|GetActorLocation)) (Utilities|Time|GetWorldDeltaSeconds) 0.0))
    (CallFunction|RotationLoop)
    (Utilities|FlowControl|DoOnce false :!label _label
      (:Completed
        (Utilities|FlowControl|Sequence
          (:then_0
            (Animation|PlayAnimMontage "/Game/Mannequin/Animations/Caught.Caught" 1.0 "None")
            (Utilities|FlowControl|Delay 1.0)
            (CameraFades|StartCameraFade :self (Game|GetPlayerCameraManager 0) :ToAlpha 1.0 :Duration 2.0 :bShouldFadeAudio true :bHoldWhenFinished true)
            (Utilities|FlowControl|Delay 2.1)
            (bind _returnvalue_2 (Game|GetCurrentLevelName true))
            (Game|OpenLevel(byName) (Utilities|String|StringToName _returnvalue_2))
            (Variables|Default|SetCaught? false))
          (:then_1
            (Utilities|FlowControl|Delay 0.5)
            (Variables|Default|SetShouldLoop? false)
            (goto _label Reset)))))))

(event Custom|RandomRoam
  ;[1 1 1] Roam
  (if (not (Variables|Default|GetCaught?))
    (AI|AIMoveTo self (.RandomLocation (AI|Navigation|GetRandomReachablePointinRadius (Transformation|GetActorLocation) 1.5e+03 0 0)) 0 5.0 false
      (:OnSuccess
        (Utilities|FlowControl|Delay (Math|Random|RandomFloatinRange 1.0 3.0)))
      (:OnFail
        _))
    (if (not (Variables|Default|GetInvestigating?))
      (CallFunction|RandomRoam))))

(event Collision|EventActorBeginOverlap
  (params (OtherActor :type Actor%20Object%20Reference)))

(event EventTick
  (params (DeltaSeconds :type Float%20%28single-precision%29))
  ;[1 1 1] Chase
  (if (not (Variables|Default|GetCan%20See%20Enemy))
    (Utilities|FlowControl|Delay 0.4)
    (if (not (Variables|Default|GetCan%20See%20Enemy))
      (Audio|Components|Audio|FadeOut (Variables|Default|GetAudio) 5.0 0.0 "Linear" :!class /Script/Engine.AudioComponent)
      (Utilities|FlowControl|DoOnce false) ; enters at Reset
    )))

(event EventBeginPlay
  ;[1 1 1] Create Audio Reference
  (CallFunction|RandomRoam)
  (bind _returnvalue (AddComponent|AddAudioComponent false))
  (Audio|Components|Audio|Stop _returnvalue)
  (Variables|Default|SetAudio _returnvalue))

(fn ConstructionScript)