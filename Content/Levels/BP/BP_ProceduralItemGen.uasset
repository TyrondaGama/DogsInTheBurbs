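; BP_ProceduralItemGen is a level actor that randomizes the look of three obstacle meshes.
; Its construction script applies the NewTransform variable to the Scene component, then gives each obstacle a random mesh from MeshLibrary01.
; The first obstacle draws from a narrower index range than the other two.
; The picks use unseeded random integers, so they re-roll whenever construction reruns, and the event graph has no active logic.
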(event EventBeginPlay)

(event Collision|EventActorBeginOverlap
  (params (OtherActor :type Actor%20Object%20Reference)))

(event EventTick
  (params (DeltaSeconds :type Float%20%28single-precision%29)))

(fn ConstructionScript
  (Transformation|SetRelativeTransform (Variables|Default|GetScene) (Variables|Default|GetNew%20Transform) false false)
  (Components|StaticMesh|SetStaticMesh (Variables|Default|GetObstacle) (Utilities|Array|Get(acopy) (Variables|Default|GetMeshLibrary01) (Math|Random|RandomIntegerinRange 0 1)))
  (Components|StaticMesh|SetStaticMesh (Variables|Default|GetObstacle01) (Utilities|Array|Get(acopy) (Variables|Default|GetMeshLibrary01) (Math|Random|RandomIntegerinRange 0 4)))
  (Components|StaticMesh|SetStaticMesh (Variables|Default|GetObstacle02) (Utilities|Array|Get(acopy) (Variables|Default|GetMeshLibrary01) (Math|Random|RandomIntegerinRange 0 4))))